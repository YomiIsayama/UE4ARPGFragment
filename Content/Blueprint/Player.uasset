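; Player character with camera-relative movement that switches between a bow and a two-handed melee weapon.
; Keys 1 and 2 play equip montages, move weapons between body and hand sockets after delays, and update State and Animation.
; Left click cycles four melee attacks or fires the arrow that Tick keeps spawned on a socket in bow state.
; Right click draws the bow, turns the character with the controller and shifts the spring arm via timeline.
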(event Custom|TakeOutWeapon
  (params (IsBow :type Boolean))
  (if IsBow
    (Animation|PlayAnimMontage "/Game/Mannequin/Archer/Animations/InPlace/Bow_InPlace_Equip_Montage.Bow_InPlace_Equip_Montage" 1.0 "None")
    (Utilities|FlowControl|Delay 1.8)
    (Transformation|AttachComponentToComponent (Variables|Default|GetBow) (Variables|Character|GetMesh) "BowHand" "SnapToTarget" "SnapToTarget" "SnapToTarget" true)
    (Variables|Default|Setstate 1.0)
    (else
      (Animation|PlayAnimMontage "/Game/Mannequin/TwoHandSword/InPlace/2Handed_InPlace_EquipBack_Montage.2Handed_InPlace_EquipBack_Montage" 1.0 "None")
      (Utilities|FlowControl|Delay 1.6)
      (Transformation|AttachComponentToComponent (Variables|Default|GetMeleeWeapon) (Variables|Character|GetMesh) "MeleeHand" "SnapToTarget" "SnapToTarget" "SnapToTarget" true)
      (Variables|Default|Setstate 2.0))))

(event Custom|TakeBackWeapon
  (params (IsBow :type Boolean))
  (if IsBow
    (Animation|PlayAnimMontage "/Game/Mannequin/Archer/Animations/InPlace/Bow_InPlace_Unequip_Montage.Bow_InPlace_Unequip_Montage" 1.0 "None")
    (Utilities|FlowControl|Delay 1.8)
    (Transformation|AttachComponentToComponent (Variables|Default|GetBow) (Variables|Character|GetMesh) "Bow" "SnapToTarget" "SnapToTarget" "SnapToTarget" true)
    (else
      (Animation|PlayAnimMontage "/Game/Mannequin/TwoHandSword/InPlace/2Handed_InPlace_UnequipBack_Montage.2Handed_InPlace_UnequipBack_Montage" 1.0 "None")
      (Utilities|FlowControl|Delay 1.9)
      (Transformation|AttachComponentToComponent (Variables|Default|GetMeleeWeapon) (Variables|Character|GetMesh) "Melee" "SnapToTarget" "SnapToTarget" "SnapToTarget" true))))

(event EventBeginPlay)

(event Collision|EventActorBeginOverlap
  (params (OtherActor :type Actor%20Object%20Reference)))

(event EventTick
  (params (DeltaSeconds :type Float%20%28single-precision%29))
  (Utilities|FlowControl|Sequence
    (:then_0
      (if (== (Variables|Default|Getstate) 1.0)
        (if (not (Variables|Default|GetIsArrow))
          (bind _returnvalue (Game|SpawnActorfromClass "/Game/Blueprint/Arrow.Arrow_C" (Math|Transform|MakeTransform "0, 0, 0" "0, 0, 0" "1,1,1") "Undefined" 0 0))
          (Transformation|AttachComponentToComponent _returnvalue (Variables|Character|GetMesh) "Arrow" "SnapToTarget" "SnapToTarget" "SnapToTarget" true)
          (Variables|Default|SetIsArrow true))
        (elif (Variables|Default|GetIsArrow)
          (Transformation|DetachFromComponent (Variables|/Script/Engine.Actor|GetRootComponent _returnvalue) "KeepRelative" "KeepRelative" "KeepRelative" true)
          (Variables|Default|SetIsArrow false))))))

(event Input|AxisEvents|InputAxisMoveForward
  (params (AxisValue :type Float%20%28single-precision%29))
  (Pawn|Input|AddMovementInput (Math|Vector|GetForwardVector (Math|Rotator|MakeRotator 0.0 0.0 (.Yaw (Math|Rotator|BreakRotator (Pawn|GetControlRotation :!class /Script/Engine.Pawn))))) AxisValue false))

(event Input|AxisEvents|InputAxisMoveRight
  (params (AxisValue :type Float%20%28single-precision%29))
  (Pawn|Input|AddMovementInput (Math|Vector|GetRightVector (Math|Rotator|MakeRotator 0.0 0.0 (.Yaw (Math|Rotator|BreakRotator (Pawn|GetControlRotation :!class /Script/Engine.Pawn))))) AxisValue false))

(event Input|AxisEvents|InputAxisLookUp
  (params (AxisValue :type Float%20%28single-precision%29))
  (Pawn|Input|AddControllerPitchInput AxisValue))

(event Input|AxisEvents|InputAxisTurn
  (params (AxisValue :type Float%20%28single-precision%29))
  (Pawn|Input|AddControllerYawInput AxisValue))

(event Input|MouseEvents|LeftMouseButton
  (params (Key :type Key%20Structure :default "None"))
  (:Pressed
    (if (== (Variables|Default|Getstate) 2.0)
      (if (Variables|Default|GetCanAttack)
        (Variables|Default|SetCanAttack false)
        (Animation|PlayAnimMontage (Utilities|Select :Index (Variables|Default|GetID) :Option%200 "/Game/Mannequin/TwoHandSword/RootMotion/2Handed_Attack_04_Montage.2Handed_Attack_04_Montage" :Option%201 "/Game/Mannequin/TwoHandSword/RootMotion/2Handed_Attack_05_Montage.2Handed_Attack_05_Montage" :Option%202 "/Game/Mannequin/TwoHandSword/RootMotion/2Handed_Attack_07_Montage.2Handed_Attack_07_Montage" :Option%203 "/Game/Mannequin/TwoHandSword/RootMotion/2Handed_Attack_12_Montage.2Handed_Attack_12_Montage") 1.0 "None")
        (Math|Integer|CompareInt (Variables|Default|GetID) 3
          (:>
            (Variables|Default|SetID 0 :!label _label))
          (:==
            (goto _label))
          (:<
            (Variables|Default|SetID (+ (Variables|Default|GetID) 1)))))
      (elif (== (Variables|Default|Getstate) 1.0)
        (if (Variables|Default|GetCanAttack)
          (if (Variables|Default|GetBow%20Pull)
            (Variables|Default|SetCanAttack false)
            (Transformation|DetachFromActor (stale EventTick _returnvalue) "KeepWorld" "KeepWorld" "KeepWorld")
            (Default|Fire (stale EventTick _returnvalue))
            (Animation|PlayAnimMontage "/Game/Mannequin/Archer/Animations/InPlace/Bow_InPlace_Shoot_2_Aim_Montage.Bow_InPlace_Shoot_2_Aim_Montage" 1.0 "None")
            (Animation|Montage|MontagePlay (Components|SkeletalMesh|GetAnimInstance (Variables|Default|GetBow)) "/Game/Mannequin/Archer/Animations/Bow/Bow_Shoot_2_Idle_02_Bow_Montage.Bow_Shoot_2_Idle_02_Bow_Montage" 1.0 "MontageLength" 0.0 true)
            (Variables|Default|SetIsArrow false)))))))

(event Input|MouseEvents|RightMouseButton
  (params (Key :type Key%20Structure :default "None"))
  (bind _charactermovement (Variables|Character|GetCharacterMovement))
  (:Pressed
    (Utilities|FlowControl|Sequence
      (:then_0
        (if (== (Variables|Default|Getstate) 1.0)
          (if (Variables|Default|GetCanAttack)
            (Variables|Default|SetBow%20Pull true)
            (Utilities|FlowControl|Sequence
              (:then_1
                (Variables|/Script/Engine.CharacterMovementComponent|SetbUseControllerDesiredRotation _charactermovement true)
                (Variables|/Script/Engine.CharacterMovementComponent|SetbOrientRotationToMovement _charactermovement false)
                (bind _newtrack_0 (Timeline|Timeline_0 Play)
                  (:Update
                    (Variables|/Script/Engine.SpringArmComponent|SetSocketOffset (Variables|Default|GetSpringArm) _newtrack_0))))))))))
  (:Released
    (Variables|Default|SetBow%20Pull false)
    (Variables|/Script/Engine.CharacterMovementComponent|SetbUseControllerDesiredRotation _charactermovement false)
    (Variables|/Script/Engine.CharacterMovementComponent|SetbOrientRotationToMovement _charactermovement true)
    (Timeline|Timeline_0 Reverse)))

(event Input|KeyboardEvents|1
  (params (Key :type Key%20Structure :default "None"))
  (:Pressed
    (if (Variables|Default|GetCanAttack)
      (Variables|Default|SetCanAttack false)
      (if (== (Variables|Default|Getstate) 1.0)
        (CallFunction|TakeBackWeapon true)
        (Variables|Default|Setstate 0.0)
        (Variables|Default|SetAnimation "NewEnumerator0")
        (elif (== (Variables|Default|Getstate) 0.0)
          (CallFunction|TakeoutWeapon true)
          (Variables|Default|Setstate 2.0)
          (Variables|Default|SetAnimation "NewEnumerator2")
          (elif (== (Variables|Default|Getstate) 2.0)
            (CallFunction|TakeBackWeapon false)
            (Variables|Default|Setstate 0.0)
            (CallFunction|TakeoutWeapon true)
            (Variables|Default|SetAnimation "NewEnumerator2")))))))

(event Input|KeyboardEvents|2
  (params (Key :type Key%20Structure :default "None"))
  (:Pressed
    (if (Variables|Default|GetCanAttack)
      (Variables|Default|SetCanAttack false)
      (if (== (Variables|Default|Getstate) 2.0)
        (CallFunction|TakeBackWeapon false)
        (Variables|Default|Setstate 0.0)
        (Variables|Default|SetAnimation "NewEnumerator0")
        (elif (== (Variables|Default|Getstate) 0.0)
          (CallFunction|TakeoutWeapon false)
          (Variables|Default|Setstate 1.0)
          (Variables|Default|SetAnimation "NewEnumerator1")
          (elif (== (Variables|Default|Getstate) 1.0)
            (CallFunction|TakeBackWeapon true)
            (Variables|Default|Setstate 0.0)
            (CallFunction|TakeoutWeapon false)
            (Variables|Default|SetAnimation "NewEnumerator1")))))))

(fn ConstructionScript
  (Transformation|AttachComponentToComponent (Variables|Default|GetMeleeWeapon) (Variables|Character|GetMesh) "Melee" "SnapToTarget" "SnapToTarget" "SnapToTarget" true)
  (Transformation|AttachComponentToComponent (Variables|Default|GetBow) (Variables|Character|GetMesh) "Bow" "SnapToTarget" "SnapToTarget" "SnapToTarget" true)
  (Transformation|AttachComponentToComponent (Variables|Default|GetQuiver) (Variables|Character|GetMesh) "Quiver" "SnapToTarget" "SnapToTarget" "SnapToTarget" true))